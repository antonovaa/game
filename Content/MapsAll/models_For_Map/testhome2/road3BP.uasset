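; Road Blueprint in a test map that moves its static mesh to a fixed raised, sideways offset and back.
; BeginPlay caches the mesh's starting world location, waits briefly, then plays a timeline that lerps the position using its Updawn track, without sweep.
; When the timeline finishes, it prints debug state (direction, alpha, start and current locations) and calls Reverse to send the mesh back.
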(event EventBeginPlay
  (bind _staticmesh (Variables|Default|GetStaticMesh))
  (Variables|Default|SetstartLocal (Transformation|GetWorldLocation _staticmesh))
  (Utilities|FlowControl|Delay 1.0)
  (bind (_direction _updawn) (Timeline|Timeline_toupdawn Play)
    (:Update
      (Transformation|SetWorldLocation _staticmesh (Math|Vector|Lerp(Vector) (Variables|Default|GetstartLocal) (+ (Variables|Default|GetstartLocal) "-777.000000,1650.000000,3300.000000") _updawn) false false))
    (:Finished
      (Development|PrintString (Utilities|String|Append (Utilities|String|EnumtoString _direction) "---" (Utilities|String|ToString(Float) _updawn) "---" (Utilities|String|ToString(Vector) (Variables|Default|GetstartLocal)) "---" (Utilities|String|ToString(Vector) (Math|Vector|Lerp(Vector) (Variables|Default|GetstartLocal) (+ (Variables|Default|GetstartLocal) "-777.000000,1650.000000,3300.000000") _updawn))) true true "(R=0.000000,G=0.660000,B=1.000000,A=1.000000)" 0.0)
      (Timeline|Timeline_toupdawn Reverse))))

(event Collision|EventActorBeginOverlap
  (params (OtherActor :type Actor%20Object%20Reference)))

(event EventTick
  (params (DeltaSeconds :type Float%20%28single-precision%29)))

(fn ConstructionScript)